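; Game mode for a timed typing game that manages the word queue, per-word scoring and game over.
; Once the start HUD hides, Tick fills a seven-word queue with unique random Data Table entries and replaces each completed word.
; Word points decay through a Delay on Tick and add to MainController's score on completion.
; Helper functions track typed and untyped letters, while a looping timer counts seconds toward the time limit.
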(event Custom|PointsCountDown
  (if (> (Variables|Default|GetPoints) 0)
    (Utilities|FlowControl|Delay 0.2)
    (Variables|Default|SetPoints (- (Variables|Default|GetPoints) 1))))

(event Custom|StartTimer
  (bind _returnvalue (Utilities|Time|SetTimerbyFunctionName self "CalculateElapsedTime" 1.0 true))
  (Variables|Default|SetElapsed%20time (Class|KismetSystemLibrary|GetTimerElapsedTimeHandle _returnvalue)))

(event EventTick
  (params (DeltaSeconds :type Float%20%28single-precision%29))
  (bind _asmain_controller (Utilities|Casting|CastToMainController (Game|GetPlayerController 0)))
  (if (not (Widget|IsVisible (Variables|/Game/Blueprints/MainController.MainController_C|GetHudGameStart _asmain_controller)))
    (CallFunction|CheckGameOver)
    (if (< (Variables|Default|GetNoOfActiveWords) 7)
      (CallFunction|SpawnWord :!label _label)
      (CallFunction|GetActiveWord)
      (CallFunction|GetActiveLetter)
      (Variables|Default|SetPoints 20)
      (else
        (bind _complete_ (CallFunction|IsWordComplete?))
        (if _complete_
          (bind _asmain_controller_2 (Utilities|Casting|CastToMainController (Game|GetPlayerController 0)))
          (Variables|/Game/Blueprints/MainController.MainController_C|SetPoints _asmain_controller_2 (+ (Variables|/Game/Blueprints/MainController.MainController_C|GetPoints _asmain_controller_2) (Variables|Default|GetPoints)))
          (Variables|Default|SetWordsCompleted (+ (Variables|Default|GetWordsCompleted) 1))
          (goto _label)
          (else
            (CallFunction|PointsCountDown)))))))

(fn ConstructionScript)

(fn SpawnWord
  (bind _activewords (Variables|Default|GetActiveWords))
  (Variables|Default|SetWordExists? false :!label _label)
  (bind _outrownames (DataTable|GetDataTableRowNames "/Game/Blueprints/ListOfWords.ListOfWords"))
  (bind _returnvalue (Utilities|GetDataTableRow "/Game/Blueprints/ListOfWords.ListOfWords" (Utilities|String|StringToName (Utilities|String|Append "E" (Utilities|String|ToString(Integer) (Math|Random|RandomIntegerinRange 0 (Utilities|Array|Length _outrownames))))))
    (:then
      (for _array_element (Variables|Default|GetActiveWords)
        (if (Utilities|Enum|Equal(Enum) _array_element (.Word (Utilities|Struct|BreakWords _returnvalue)))
          (Variables|Default|SetWordExists? true)))
      (if (Variables|Default|GetWordExists?)
        (goto _label)
        (else
          (Utilities|Array|Add _activewords (.Word (Utilities|Struct|BreakWords _returnvalue)))
          (Variables|Default|SetNoOfActiveWords (Utilities|Array|Length _activewords)))))))

(fn GetActiveLetter
  (Variables|Default|SetActiveLetter (Utilities|Array|Get(acopy) (Utilities|String|GetCharacterArrayfromString (Variables|Default|GetCurrentWord)) (Variables|Default|GetLettersComplete))))

(fn GetActiveWord
  (bind _output_get (Variables|Default|SetCurrentWord (Utilities|Array|Get(acopy) (Variables|Default|GetActiveWords))))
  (bind _output_get_2 (Variables|Default|SetNotTypedArray (Utilities|String|GetCharacterArrayfromString _output_get)))
  (Variables|Default|SetNotTypedString (Utilities|String|JoinStringArray _output_get_2 (Variables|Default|GetBlankString))))

(fn IsWordComplete?
  (if (== (Utilities|Array|Length (Utilities|String|GetCharacterArrayfromString (Variables|Default|GetCurrentWord))) (Variables|Default|GetLettersComplete))
    (Utilities|Array|RemoveIndex (Variables|Default|GetActiveWords))
    (Variables|Default|SetLettersComplete 0)
    (Variables|Default|SetTypedString "")
    (return true)
    (else
      (return false))))

(fn GetTypedLetters
  (params (InputKey :type String))
  (Variables|Default|SetTypedString (Utilities|String|Append (Variables|Default|GetTypedString) InputKey)))

(fn GetNotTypedLetters
  (bind _nottypedarray (Variables|Default|GetNotTypedArray))
  (Utilities|Array|RemoveIndex _nottypedarray)
  (Variables|Default|SetNotTypedString (Utilities|String|JoinStringArray _nottypedarray (Variables|Default|GetBlankString))))

(fn CalculateElapsedTime
  (Math|Float|IncrementFloat (Variables|Default|GetElapsed%20time)))

(fn CheckGameOver
  (if (>= (Variables|Default|GetElapsed%20time) (Variables|Default|GetTimeLimit))
    (bind _asmain_controller (Utilities|Casting|CastToMainController (Game|GetPlayerController 0)))
    (Widget|SetVisibility (Variables|/Game/Blueprints/MainController.MainController_C|GetHudGameOver _asmain_controller) "Visible")
    (Widget|SetVisibility (Variables|/Game/Blueprints/MainController.MainController_C|GetHudMain _asmain_controller) "Hidden")))