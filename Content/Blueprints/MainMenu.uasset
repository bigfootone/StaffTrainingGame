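; MainMenu is an actor Blueprint for the main menu that sets up the initial menu state and can print saved Endless-mode high scores.
; On BeginPlay it casts the player controller to MainMenuController and hides its GameModeSelect element.
; A separate CheckHighscores event loads the EndlessScores save slot as HighScores and prints each name and score as debug strings.
; That event also creates a HighScores save object, which goes unused.
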(event Custom|CheckHighscores
  (SaveGame|CreateSaveGameObject "/Game/Blueprints/HighScores.HighScores_C")
  (bind _returnvalue (SaveGame|LoadGamefromSlot "EndlessScores"))
  (bind _output_get (Variables|Default|SetSaveGameInstance _returnvalue))
  (bind _ashigh_scores (Utilities|Casting|CastToHighScores _output_get))
  (for _array_element (Variables|/Game/Blueprints/HighScores.HighScores_C|GetScoresEndless _ashigh_scores)
    (Development|PrintString (Utilities|String|Append (.Name (Utilities|Struct|BreakHighscoreSetup _array_element)) " :" (Utilities|String|ToString(Integer) (.Score (Utilities|Struct|BreakHighscoreSetup _array_element)))))))

(event EventBeginPlay
  (bind _asmain_menu_controller (Utilities|Casting|CastToMainMenuController (Game|GetPlayerController 0)))
  (Widget|SetVisibility (Variables|/Game/Blueprints/MainMenuController.MainMenuController_C|GetGameModeSelect _asmain_menu_controller) "Hidden"))

(fn ConstructionScript)