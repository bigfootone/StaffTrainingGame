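; Main menu controller Blueprint that builds the menu UI when play begins.
; BeginPlay creates the main menu, game mode selection and leaderboard widgets, stores each in a variable and adds it to the viewport.
; The leaderboard is hidden immediately, while the other two widgets keep their default visibility.
; It has no Tick or construction logic.
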(event EventBeginPlay
  (bind _returnvalue (UserInterface|CreateWidget "/Game/Blueprints/UI/HudMainMenu.HudMainMenu_C" (Game|GetPlayerController 0)))
  (bind _output_get (Variables|Default|SetHudMainMenu _returnvalue))
  (UserInterface|Viewport|AddtoViewport _output_get 0)
  (bind _returnvalue_2 (UserInterface|CreateWidget "/Game/Blueprints/UI/SelectGameMode.SelectGameMode_C" (Game|GetPlayerController 0)))
  (bind _output_get_2 (Variables|Default|SetGameModeSelect _returnvalue_2))
  (UserInterface|Viewport|AddtoViewport _output_get_2 0)
  (bind _returnvalue_3 (UserInterface|CreateWidget "/Game/Blueprints/UI/Leaderboards.Leaderboards_C"))
  (bind _output_get_3 (Variables|Default|SetHudLeaderboard _returnvalue_3))
  (UserInterface|Viewport|AddtoViewport _output_get_3 0)
  (Widget|SetVisibility _output_get_3 "Hidden"))

(event EventTick
  (params (DeltaSeconds :type Float%20%28single-precision%29)))

(fn ConstructionScript)