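; Player controller that manages the main UI and saves high scores for Endless mode.
; On BeginPlay it adds the HUD, a hidden game-over screen and a start screen, and Tick shows the mouse cursor whenever the HUD is not visible.
; SaveGameEndless loads the EndlessScores slot, inserts the new name and score above the first lower score, or appends it while under ten entries, then saves.
; The list is never trimmed here.
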(event Custom|SaveGameEndless
  (params (Score :type Integer) (name :type String))
  (bind _highscoresetup (Utilities|Struct|MakeHighscoreSetup name Score))
  (SaveGame|CreateSaveGameObject "/Game/Blueprints/HighScores.HighScores_C")
  (bind _returnvalue (SaveGame|LoadGamefromSlot "EndlessScores"))
  (bind _ashigh_scores (Utilities|Casting|CastToHighScores _returnvalue))
  (bind _output_get (Variables|Default|SetHighScoreSaves _ashigh_scores))
  (if (> (Utilities|Array|Length (Variables|/Game/Blueprints/HighScores.HighScores_C|GetScoresEndless _output_get)) 0)
    (bind (_array_element _array_index) (Utilities|Array|ForEachLoopwithBreak (Variables|/Game/Blueprints/HighScores.HighScores_C|GetScoresEndless _output_get))
      (:LoopBody
        (if (< (.Score (Utilities|Struct|BreakHighscoreSetup _array_element)) Score)
          (Utilities|Array|Insert (Variables|/Game/Blueprints/HighScores.HighScores_C|GetScoresEndless _output_get) _highscoresetup _array_index)
          (CallFunction|BreakHighscoreLoop)
          (Variables|Default|SetAdded? true)))
      (:Completed
        (if (< (Utilities|Array|Length (Variables|/Game/Blueprints/HighScores.HighScores_C|GetScoresEndless _output_get)) 10)
          (if (Variables|Default|GetAdded?)
            _
            (else
              (Utilities|Array|Add (Variables|/Game/Blueprints/HighScores.HighScores_C|GetScoresEndless _output_get) _highscoresetup)
              (Variables|Default|SetAdded? false))))
        (SaveGame|SaveGametoSlot (Variables|Default|GetHighScoreSaves) "EndlessScores" :!label _label)))
    (else
      (Utilities|Array|Insert (Variables|/Game/Blueprints/HighScores.HighScores_C|GetScoresEndless _output_get) _highscoresetup)
      (goto _label))))

(event Custom|BreakHighscoreLoop
  (Utilities|Array|ForEachLoopwithBreak (Variables|/Game/Blueprints/HighScores.HighScores_C|GetScoresEndless (stale Custom|SaveGameEndless _output_get))) ; enters at Break
)

(event EventBeginPlay
  (bind _returnvalue (Game|GetPlayerController 0))
  (bind _returnvalue_2 (UserInterface|CreateWidget "/Game/Blueprints/UI/HudMain.HudMain_C" _returnvalue))
  (bind _output_get (Variables|Default|SetHudMain _returnvalue_2))
  (UserInterface|Viewport|AddtoViewport _output_get 0)
  (bind _returnvalue_3 (UserInterface|CreateWidget "/Game/Blueprints/UI/GameOverScreenEndless.GameOverScreenEndless_C" _returnvalue))
  (bind _output_get_2 (Variables|Default|SetHudGameOver _returnvalue_3))
  (UserInterface|Viewport|AddtoViewport _output_get_2 0)
  (Widget|SetVisibility _output_get_2 "Hidden")
  (bind _returnvalue_4 (UserInterface|CreateWidget "/Game/Blueprints/UI/GameStart.GameStart_C"))
  (bind _output_get_3 (Variables|Default|SetHudGameStart _returnvalue_4))
  (UserInterface|Viewport|AddtoViewport _output_get_3 0))

(event EventTick
  (params (DeltaSeconds :type Float%20%28single-precision%29))
  (if (Widget|IsVisible (Variables|Default|GetHudMain))
    (Variables|Default|SetbShowMouseCursor false)
    (else
      (Variables|Default|SetbShowMouseCursor true))))

(fn ConstructionScript)