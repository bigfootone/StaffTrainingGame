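; Player pawn that handles keyboard input for a typing mechanic driven by BuildGameMode.
; It enables input for the first player controller on BeginPlay, then compares each pressed key's display name with the game mode's active letter.
; On a match it increments the completed letter count and calls the game mode's active, typed and not-typed letter functions.
; Non-matching keys have no effect.
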(event EventBeginPlay
  (Input|EnableInput (Game|GetPlayerController 0)))

(event Input|KeyboardEvents|AnyKey
  (params (Key :type Key%20Structure :default "AnyKey"))
  (bind _returnvalue (Class|KismetInputLibrary|KeyGetDisplayName Key))
  (:Pressed
    (bind _asbuild_game_mode (Utilities|Casting|CastToBuildGameMode (Game|GetGameMode)))
    (if (Utilities|Enum|Equal(Enum) _returnvalue (Utilities|Text|ToText(String) (Variables|/Game/Blueprints/BuildGameMode.BuildGameMode_C|GetActiveLetter _asbuild_game_mode)))
      (bind _asbuild_game_mode_2 (Utilities|Casting|CastToBuildGameMode (Game|GetGameMode)))
      (Math|Integer|IncrementInt (Variables|/Game/Blueprints/BuildGameMode.BuildGameMode_C|GetLettersComplete _asbuild_game_mode_2)
        (:%20%20
          (Default|GetActiveLetter _asbuild_game_mode_2)
          (Default|GetTypedLetters _asbuild_game_mode_2 (Utilities|String|ToString(Text) _returnvalue))
          (Default|GetNotTypedLetters _asbuild_game_mode_2))))))

(fn ConstructionScript)